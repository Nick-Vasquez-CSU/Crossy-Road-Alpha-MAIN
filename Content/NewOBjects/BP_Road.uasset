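; BP_Road is a road segment actor that triggers spawning of further road and cars as actors overlap it.
; A player entering NewRoad_COLLIDE makes RoadSpawner spawn a road, while a BP_RoadSpawner entering Car_Respawn spawns a car at CarSPAWN, then gets destroyed.
; RandomRoad, uncalled here, picks one of four grass, lane, water or railroad meshes, flips it, and returns a separately evaluated random index.
; Tick draws a "Roads" text label.
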(event OnComponentBeginOverlap(NewRoad_COLLIDE)
  (params (OverlappedComponent :type Primitive%20Component%20Object%20Reference) (OtherActor :type Actor%20Object%20Reference) (OtherComp :type Primitive%20Component%20Object%20Reference) (OtherBodyIndex :type Integer) (bFromSweep :type Boolean) (SweepResult :type Hit%20Result%20Structure%20%28by%20ref%29))
  (Utilities|Casting|CastToBP_Player OtherActor)
  (Default|SpawnRoadatSpawnpoint (Variables|Default|GetRoadSpawner)))

(event OnComponentBeginOverlap(Car_Respawn)
  (params (OverlappedComponent :type Primitive%20Component%20Object%20Reference) (OtherActor :type Actor%20Object%20Reference) (OtherComp :type Primitive%20Component%20Object%20Reference) (OtherBodyIndex :type Integer) (bFromSweep :type Boolean) (SweepResult :type Hit%20Result%20Structure%20%28by%20ref%29))
  (bind _asbp_road_spawner (Utilities|Casting|CastToBP_RoadSpawner OtherActor))
  (Default|SpawnCar _asbp_road_spawner (Transformation|GetWorldLocation (Variables|Default|GetCar_SPAWN)))
  (Actor|DestroyActor OtherActor))

(event EventBeginPlay)

(event Collision|EventActorBeginOverlap
  (params (OtherActor :type Actor%20Object%20Reference)))

(event EventTick
  (params (DeltaSeconds :type Float%20%28single-precision%29))
  (Class|WidgetBlueprintLibrary|DrawTextFormatted :Text (Variables|Default|GetRoads)))

(fn ConstructionScript)

(fn RandomRoad
  (bind _returnvalue (Math|Random|RandomIntegerinRange 0 3))
  (bind _returnvalue_2 (+ _returnvalue 0))
  (Components|StaticMesh|SetStaticMesh (Variables|Default|GetRoad) (Utilities|Select :Index _returnvalue_2 :Option%200 "/Game/NewOBjects/Grass-D_NEW.Grass-D_NEW" :Option%201 "/Game/Objects/1lane_grass.1lane_grass" :Option%202 "/Game/Objects/1lane_water_vox.1lane_water_vox" :Option%203 "/Game/Objects/railroad_vox.railroad_vox"))
  (Transformation|AddLocalRotation (Variables|Default|GetRoad) (Math|Rotator|MakeRotator 1.8e+02 0.0 0.0) false false)
  (return _returnvalue_2))