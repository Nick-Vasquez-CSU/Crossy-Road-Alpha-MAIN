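; BP_Car is a moving obstacle that drives along its local offset each tick and quits the game when its Box overlaps BP_Player.
; A player overlap on the CheckSpeedUp trigger sets CarSpeed to a fixed X velocity.
; SetCar selects a vehicle, coin, log or train mesh by type, rotating the train, and stores the type for RetrieveCarType.
; SpeedUp reports whether the player and car share the same world Y.
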(event OnComponentBeginOverlap(Box)
  (params (OverlappedComponent :type Primitive%20Component%20Object%20Reference) (OtherActor :type Actor%20Object%20Reference) (OtherComp :type Primitive%20Component%20Object%20Reference) (OtherBodyIndex :type Integer) (bFromSweep :type Boolean) (SweepResult :type Hit%20Result%20Structure%20%28by%20ref%29))
  (Utilities|Casting|CastToBP_Player OtherActor)
  (Game|QuitGame 0 "Quit" false))

(event OnComponentBeginOverlap(CheckSpeedUp)
  (params (OverlappedComponent :type Primitive%20Component%20Object%20Reference) (OtherActor :type Actor%20Object%20Reference) (OtherComp :type Primitive%20Component%20Object%20Reference) (OtherBodyIndex :type Integer) (bFromSweep :type Boolean) (SweepResult :type Hit%20Result%20Structure%20%28by%20ref%29))
  (Utilities|Casting|CastToBP_Player OtherActor)
  (Variables|Default|SetCarSpeed "200.000000, 0, 0"))

(event EventTick
  (params (DeltaSeconds :type Float%20%28single-precision%29))
  (Transformation|AddActorLocalOffset (* (Variables|Default|GetCarSpeed) DeltaSeconds) false false))

(fn ConstructionScript)

(fn SetCar
  (params (CarType :type Integer))
  (Components|StaticMesh|SetStaticMesh (Variables|Default|GetCar) (Utilities|Select :Index CarType :Option%200 "/Game/NewOBjects/Vehicle_Sred_NEW.Vehicle_Sred_NEW" :Option%201 "/Game/Objects/coin_vox.coin_vox" :Option%202 "/Game/Objects/short_log_vox.short_log_vox" :Option%203 "/Game/Objects/train.train"))
  (Variables|Default|Settypeofcar CarType)
  (if (== CarType 3)
    (Transformation|AddLocalRotation (Variables|Default|GetCar) "270.000000,0.000000,0.000000" false false)))

(fn RetrieveCarType
  (return (Variables|Default|Gettypeofcar)))

(fn SpeedUp
  (return (== (.y (Transformation|GetWorldLocation (Variables|/Script/Engine.Actor|GetRootComponent (Game|Player|GetPlayerPawn 0)))) (.y (Transformation|GetWorldLocation (Variables|Default|GetCar))))))