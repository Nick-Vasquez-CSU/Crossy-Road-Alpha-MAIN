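; BP_Player is a player pawn with a Chicken component that hops and turns to face the pressed WASD key.
; MoveForward and MoveRight axes add MaxSpeed-scaled input along axes rotated 90 degrees from the actor's own.
; Tick consumes that input as a delta-time-scaled local offset without sweep, so movement ignores blocking collision.
; Key presses rotate only the Chicken, then share one raise, Delay and lower chain for the hop.
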(event EventBeginPlay)

(event Collision|EventActorBeginOverlap
  (params (OtherActor :type Actor%20Object%20Reference)))

(event EventTick
  (params (DeltaSeconds :type Float%20%28single-precision%29))
  (bind _returnvalue (Class|Pawn|ConsumeMovementInputVector))
  (Transformation|AddActorLocalOffset (* _returnvalue DeltaSeconds) false false))

(event Input|AxisEvents|InputAxisMoveForward
  (params (AxisValue :type Float%20%28single-precision%29))
  (Pawn|Input|AddMovementInput (Transformation|GetActorRightVector) (* AxisValue (Variables|Default|GetMaxSpeed)) false))

(event Input|AxisEvents|InputAxisMoveRight
  (params (AxisValue :type Float%20%28single-precision%29))
  (Pawn|Input|AddMovementInput (Math|Vector|NegateVector (Transformation|GetActorForwardVector)) (* AxisValue (Variables|Default|GetMaxSpeed)) false))

(event Input|KeyboardEvents|W
  (params (Key :type Key%20Structure :default "None"))
  (bind _chicken (Variables|Default|GetChicken))
  (:Pressed
    (Transformation|SetRelativeRotation _chicken "0.000000,-90.000000,90.000000" false false)
    (Transformation|SetRelativeLocation _chicken "0.000000,0.000000,20.000000" false false)
    (Utilities|FlowControl|Delay 0.3)
    (Transformation|SetRelativeLocation _chicken "0.000000, 0,0.000000" false false)))

(event Input|KeyboardEvents|S
  (params (Key :type Key%20Structure :default "None"))
  (bind _chicken (Variables|Default|GetChicken))
  (:Pressed
    (Transformation|SetRelativeRotation _chicken "0.000000,-270.000000,90.000000" false false)
    (Transformation|SetRelativeLocation _chicken "0.000000,0.000000,20.000000" false false)
    (Utilities|FlowControl|Delay 0.3)
    (Transformation|SetRelativeLocation _chicken "0.000000, 0,0.000000" false false)))

(event Input|KeyboardEvents|A
  (params (Key :type Key%20Structure :default "None"))
  (bind _chicken (Variables|Default|GetChicken))
  (:Pressed
    (Transformation|SetRelativeRotation _chicken "0.000000,-180.000000,90.000000" false false)
    (Transformation|SetRelativeLocation _chicken "0.000000,0.000000,20.000000" false false)
    (Utilities|FlowControl|Delay 0.3)
    (Transformation|SetRelativeLocation _chicken "0.000000, 0,0.000000" false false)))

(event Input|KeyboardEvents|D
  (params (Key :type Key%20Structure :default "None"))
  (bind _chicken (Variables|Default|GetChicken))
  (:Pressed
    (Transformation|SetRelativeRotation _chicken "0.000000,0.000000,90.000000" false false)
    (Transformation|SetRelativeLocation _chicken "0.000000,0.000000,20.000000" false false)
    (Utilities|FlowControl|Delay 0.3)
    (Transformation|SetRelativeLocation _chicken "0.000000, 0,0.000000" false false)))

(fn ConstructionScript)