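; Road spawner that builds a chain of randomized road segments at BeginPlay, each paired with a car.
; The first segment starts at the player pawn's XY at ground zero, and each later one attaches to the previous road's RoadSPAWN point.
; Each road's RandomRoad result configures its car through SetCar.
; Spawned roads and cars receive a reference back to the spawner.
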(event EventBeginPlay
  (CallFunction|SpawnInitialRoad))

(event Collision|EventActorBeginOverlap
  (params (OtherActor :type Actor%20Object%20Reference)))

(event EventTick
  (params (DeltaSeconds :type Float%20%28single-precision%29)))

(fn ConstructionScript)

(fn SpawnRoad
  (params (SpawnLocation :type Vector))
  (bind _returnvalue (Game|SpawnActorfromClass "/Game/NewOBjects/BP_Road.BP_Road_C" (Math|Transform|MakeTransform SpawnLocation "0, 0, 0" "1,1,1") "Undefined" 0 0))
  (bind _output_get (Variables|Default|SetNewest%20Road _returnvalue))
  (Variables|/Game/NewOBjects/BP_Road.BP_Road_C|SetRoadSpawner _output_get self)
  (bind _cartypefroad (Default|RandomRoad _output_get))
  (Variables|Default|SetCarChoose _cartypefroad))

(fn SpawnRoadatSpawnpoint
  (CallFunction|SpawnRoad (Transformation|GetWorldLocation (Variables|/Game/NewOBjects/BP_Road.BP_Road_C|GetRoad_SPAWN (Variables|Default|GetNewest%20Road))))
  (CallFunction|SpawnCar (Transformation|GetWorldLocation (Variables|/Game/NewOBjects/BP_Road.BP_Road_C|GetCar_SPAWN (Variables|Default|GetNewest%20Road)))))

(fn SpawnInitialRoad
  (bind _returnvalue (Game|Player|GetPlayerPawn 0))
  (bind _returnvalue_2 (Transformation|GetActorLocation _returnvalue))
  (for _index (range 0 10)
    (Utilities|IsValid (Variables|Default|GetNewest%20Road)
      (:Is%20Valid
        (CallFunction|SpawnRoadatSpawnpoint))
      (:Is%20Not%20Valid
        (CallFunction|SpawnRoad (Math|Vector|MakeVector (.x _returnvalue_2) (.y _returnvalue_2) 0.0))
        (CallFunction|SpawnCar (Math|Vector|MakeVector (- (.x _returnvalue_2) 5e+02) (.y _returnvalue_2) 0.0))))))

(fn SpawnCar
  (params (SpawnLocation :type Vector))
  (bind _returnvalue (Game|SpawnActorfromClass "/Game/NewOBjects/BP_Car.BP_Car_C" (Math|Transform|MakeTransform SpawnLocation "0, 0, 0" "1,1,1") "Undefined" 0 0))
  (bind _output_get (Variables|Default|SetNewest%20Car _returnvalue))
  (Variables|/Game/NewOBjects/BP_Car.BP_Car_C|SetRoadSpawner _output_get self)
  (Default|SetCar _output_get (Variables|Default|GetCarChoose)))